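; Lucy_BP is an NPC Blueprint that shows an interaction prompt when the player character enters its Box trigger.
; Overlap enables input and, unless both dialogue flags are set, creates the Interactable widget and opens a Gate.
; Leaving the box removes the widget and closes the Gate.
; The Interact press feeds that Gate, but nothing is wired after it, so no dialogue runs here.
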(event `InputAction|Interact` :consume false
  (params (Key :type "Key Structure"))
  (:`Pressed`
    (`/Engine/EditorBlueprintResources/StandardMacros.Gate` true :!label _label)))

(event `self.Box.OnComponentBeginOverlap`
  (params (OverlappedComponent :type "PrimitiveComponent Object Reference") (OtherActor :type "Actor Object Reference") (OtherComp :type "PrimitiveComponent Object Reference") (OtherBodyIndex :type Integer) (bFromSweep :type Boolean) (SweepResult :type "HitResult Structure (by ref)"))
  (bind _returnvalue (`GameplayStatics.GetPlayerController` 0))
  (cast `/Game/Character/BP_StoryAdv_Character` OtherActor)
  (`self.EnableInput` _returnvalue)
  (if (`self.1stDialogue`)
    (if (not (`self.2ndDialogue`))
      (bind _returnvalue_2 (`|CreateWidget` "/Game/Widgets/Interactable_Widget.Interactable_Widget_C" _returnvalue :!label _label_2))
      (bind _output_get (set `self.InteractableWidget` _returnvalue_2))
      (`UserWidget.AddToViewport` _output_get 0)
      (goto _label :!via `Open`))
    (else
      (goto _label_2))))

(event `self.Box.OnComponentEndOverlap`
  (params (OverlappedComponent :type "PrimitiveComponent Object Reference") (OtherActor :type "Actor Object Reference") (OtherComp :type "PrimitiveComponent Object Reference") (OtherBodyIndex :type Integer))
  (cast `/Game/Character/BP_StoryAdv_Character` OtherActor)
  (`Widget.RemoveFromParent` (`self.InteractableWidget`))
  (goto _label :!via `Close`))

(fn `UserConstructionScript`)