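; Steve NPC that plays two voiced dialogues when the player interacts.
; Box overlap with the story character shows a prompt and opens an input gate, unless both dialogue flags are set.
; The flags select the line, which locks player input for a fixed delay; the second then plays the BarBlockVolume sequence and shows the investigate-bar widget.
; Tick sets the flags from the player's FoundKnife and FoundGloves progress.
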(event `InputAction|Interact` :consume false
  (params (Key :type "Key Structure"))
  (bind _returnvalue (`GameplayStatics.GetPlayerController` 0))
  (bind _returnvalue_2 (`GameplayStatics.GetPlayerCharacter` 0))
  (bind _returnvalue_3 (`GameplayStatics.GetPlayerController` 0))
  (bind _returnvalue_4 (`GameplayStatics.GetPlayerCharacter` 0))
  (:`Pressed`
    (`/Engine/EditorBlueprintResources/StandardMacros.Gate` true :!label _label
      (:`Exit`
        (if (`self.1stDialogue`)
          (if (`self.2ndDialogue`)
            ;[1 1 1] 2ndDialogue
            (`WidgetLayoutLibrary.RemoveAllWidgets`)
            (`self.DisableInput` _returnvalue_4 _returnvalue_3)
            (`self.K2_SetActorRotation` _returnvalue_4 (struct :`Yaw` -50.0) false)
            (`GameplayStatics.PlaySoundAtLocation` "/Game/Audio/Dialogue/2ndInteraction/Steve2ndDialogue.Steve2ndDialogue" (`self.K2_GetActorLocation`) (struct) 1.0 1.0 0.0 null null null)
            (`KismetSystemLibrary.Delay` 22.0)
            (`self.EnableInput` _returnvalue_4 _returnvalue_3)
            (bind (_outactor _returnvalue_5) (`LevelSequencePlayer.CreateLevelSequencePlayer` "/Game/Sequences/BarBlockVolume.BarBlockVolume"))
            (`MovieSceneSequencePlayer.Play` _returnvalue_5)
            (set `self.2ndDialogue` true)
            (bind _returnvalue_6 (`|CreateWidget` "/Game/Widgets/Objectives/InvestigateBar_Widget.InvestigateBar_Widget_C" (`GameplayStatics.GetPlayerController` 0)))
            (`UserWidget.AddToViewport` _returnvalue_6 0))
          (else
            ;[1 1 1] 1stDialogue
            (`WidgetLayoutLibrary.RemoveAllWidgets`)
            (`self.DisableInput` _returnvalue_2 _returnvalue)
            (`self.K2_SetActorRotation` _returnvalue_2 (struct :`Yaw` -50.0) false)
            (`GameplayStatics.PlaySoundAtLocation` "/Game/Audio/Dialogue/1stInteraction/Steve1stDialogue.Steve1stDialogue" (`self.K2_GetActorLocation`) (struct) 1.0 1.0 0.0 null null null)
            (`KismetSystemLibrary.Delay` 18.0)
            (`self.EnableInput` _returnvalue_2 _returnvalue)
            (set `self.1stDialogue` true)))))))

(event `self.Box.OnComponentBeginOverlap`
  (params (OverlappedComponent :type "PrimitiveComponent Object Reference") (OtherActor :type "Actor Object Reference") (OtherComp :type "PrimitiveComponent Object Reference") (OtherBodyIndex :type Integer) (bFromSweep :type Boolean) (SweepResult :type "HitResult Structure (by ref)"))
  (bind _returnvalue (`GameplayStatics.GetPlayerController` 0))
  (cast `/Game/Character/BP_StoryAdv_Character` OtherActor)
  (`self.EnableInput` _returnvalue)
  (if (`self.1stDialogue`)
    (if (not (`self.2ndDialogue`))
      (bind _returnvalue_2 (`|CreateWidget` "/Game/Widgets/Interactable_Widget.Interactable_Widget_C" _returnvalue :!label _label_2))
      (bind _output_get (set `self.InteractableWidget` _returnvalue_2))
      (`UserWidget.AddToViewport` _output_get 0)
      (goto _label :!via `Open`))
    (else
      (goto _label_2))))

(event `self.Box.OnComponentEndOverlap`
  (params (OverlappedComponent :type "PrimitiveComponent Object Reference") (OtherActor :type "Actor Object Reference") (OtherComp :type "PrimitiveComponent Object Reference") (OtherBodyIndex :type Integer))
  (cast `/Game/Character/BP_StoryAdv_Character` OtherActor)
  (`Widget.RemoveFromParent` (`self.InteractableWidget`))
  (goto _label :!via `Close`))

(event `self.ReceiveTick`
  (params (DeltaSeconds :type "Float (single-precision)"))
  (bind _asbp_story_adv_character (cast `/Game/Character/BP_StoryAdv_Character` (`GameplayStatics.GetPlayerCharacter` 0)))
  (if (`/Game/Character/BP_StoryAdv_Character.FoundKnife` _asbp_story_adv_character)
    (set `self.1stDialogue` true)
    (if (`/Game/Character/BP_StoryAdv_Character.FoundGloves` _asbp_story_adv_character)
      (set `self.2ndDialogue` true))))

(fn `UserConstructionScript`)