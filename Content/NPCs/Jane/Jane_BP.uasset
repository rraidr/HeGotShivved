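; Jane NPC Blueprint that plays one of two voiced dialogues based on the player's story progress.
; Box overlap shows an interact prompt and opens a Gate for the Interact input.
; Dialogue disables player input, turns the character and waits a fixed delay matching the line.
; Tick polls the character's knife and gloves flags; finding the knife unlocks the second dialogue and lets overlap reset the DoOnce.
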(event `InputAction|Interact` :consume false
  (params (Key :type "Key Structure"))
  (bind _returnvalue (`GameplayStatics.GetPlayerController` 0))
  (bind _returnvalue_2 (`GameplayStatics.GetPlayerCharacter` 0))
  (bind _returnvalue_3 (`GameplayStatics.GetPlayerController` 0))
  (bind _returnvalue_4 (`GameplayStatics.GetPlayerCharacter` 0))
  (:`Pressed`
    (`/Engine/EditorBlueprintResources/StandardMacros.DoOnce` false :!label _label
      (:`Completed`
        (`/Engine/EditorBlueprintResources/StandardMacros.Gate` true :!label _label_2
          (:`Exit`
            (if (`self.1stDialogue`)
              (if (`self.KnifeFound`)
                ;[1 1 1] 2ndDialogue
                (`WidgetLayoutLibrary.RemoveAllWidgets`)
                (`self.DisableInput` _returnvalue_4 _returnvalue_3)
                (`self.K2_SetActorRotation` _returnvalue_4 (struct :`Yaw` -50.0) false)
                (`GameplayStatics.PlaySoundAtLocation` "/Game/Audio/Dialogue/2ndInteraction/Jane2ndDialogue.Jane2ndDialogue" (`self.K2_GetActorLocation`) (struct) 1.0 1.0 0.0 null null null)
                (`KismetSystemLibrary.Delay` 13.0)
                (`self.EnableInput` _returnvalue_4 _returnvalue_3)
                (set `self.2ndDialogue` true))
              (else
                ;[1 1 1] 1stDialogue
                (`WidgetLayoutLibrary.RemoveAllWidgets`)
                (`self.DisableInput` _returnvalue_2 _returnvalue)
                (`self.K2_SetActorRotation` _returnvalue_2 (struct :`Yaw` -120.0) false)
                (`GameplayStatics.PlaySoundAtLocation` "/Game/Audio/Dialogue/1stInteraction/Jane1stDialogue.Jane1stDialogue" (`self.K2_GetActorLocation`) (struct) 1.0 1.0 0.0 null null null)
                (`KismetSystemLibrary.Delay` 28.0)
                (`self.EnableInput` _returnvalue_2 _returnvalue)
                (set `self.1stDialogue` true)))))))))

(event `Reset Interact`
  (if (`self.KnifeFound`)
    (goto _label :!via `Reset`)))

(event `self.Box.OnComponentBeginOverlap`
  (params (OverlappedComponent :type "PrimitiveComponent Object Reference") (OtherActor :type "Actor Object Reference") (OtherComp :type "PrimitiveComponent Object Reference") (OtherBodyIndex :type Integer) (bFromSweep :type Boolean) (SweepResult :type "HitResult Structure (by ref)"))
  (bind _returnvalue (`GameplayStatics.GetPlayerController` 0))
  (cast `/Game/Character/BP_StoryAdv_Character` OtherActor)
  (`self.EnableInput` _returnvalue)
  (if (`self.1stDialogue`)
    (if (`self.KnifeFound`)
      (bind _returnvalue_2 (`|CreateWidget` "/Game/Widgets/Interactable_Widget.Interactable_Widget_C" _returnvalue :!label _label_3))
      (bind _output_get (set `self.InteractableWidget` _returnvalue_2))
      (`UserWidget.AddToViewport` _output_get 0)
      (`self.Reset Interact`)
      (goto _label_2 :!via `Open`))
    (else
      (goto _label_3))))

(event `self.Box.OnComponentEndOverlap`
  (params (OverlappedComponent :type "PrimitiveComponent Object Reference") (OtherActor :type "Actor Object Reference") (OtherComp :type "PrimitiveComponent Object Reference") (OtherBodyIndex :type Integer))
  (cast `/Game/Character/BP_StoryAdv_Character` OtherActor)
  (`Widget.RemoveFromParent` (`self.InteractableWidget`))
  (goto _label_2 :!via `Close`))

(event `self.ReceiveTick`
  (params (DeltaSeconds :type "Float (single-precision)"))
  (bind _asbp_story_adv_character (cast `/Game/Character/BP_StoryAdv_Character` (`GameplayStatics.GetPlayerCharacter` 0)))
  (if (`/Game/Character/BP_StoryAdv_Character.FoundKnife` _asbp_story_adv_character)
    (set `self.1stDialogue` true)
    (set `self.KnifeFound` true)
    (if (`/Game/Character/BP_StoryAdv_Character.FoundGloves` _asbp_story_adv_character)
      (set `self.2ndDialogue` true)
      (set `self.GlovesFound` true))))

(fn `UserConstructionScript`)