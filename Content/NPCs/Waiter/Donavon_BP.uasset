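; Donavon waiter NPC that plays one of four staged voice lines as the player finds the knife, gloves and rag.
; A trigger box shows an interact widget and opens a gate for the Interact input while dialogue is available.
; Interacting disables player input, turns the player and plays the line for a fixed delay.
; Tick mirrors the player character's clue flags, and overlap re-arms the DoOnce once a clue is found.
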(event `InputAction|Interact` :consume false
  (params (Key :type "Key Structure"))
  (bind _returnvalue (`GameplayStatics.GetPlayerCharacter` 0))
  (bind _returnvalue_2 (`GameplayStatics.GetPlayerController` 0))
  (bind _returnvalue_3 (`GameplayStatics.GetPlayerCharacter` 0))
  (bind _returnvalue_4 (`GameplayStatics.GetPlayerController` 0))
  (bind _returnvalue_5 (`GameplayStatics.GetPlayerCharacter` 0))
  (bind _returnvalue_6 (`GameplayStatics.GetPlayerController` 0))
  (bind _returnvalue_7 (`GameplayStatics.GetPlayerCharacter` 0))
  (bind _returnvalue_8 (`GameplayStatics.GetPlayerController` 0))
  ;[1 1 1] Interact
  (:`Pressed`
    (`/Engine/EditorBlueprintResources/StandardMacros.DoOnce` false :!label _label
      (:`Completed`
        (`/Engine/EditorBlueprintResources/StandardMacros.Gate` true :!label _label_2
          (:`Exit`
            (if (`self.1stDialogue`)
              (if (`self.KnifeFound`)
                (if (`self.GlovesFound`)
                  (if (`self.RagFound`)
                    ;[0 1 0.02045] 4thDialogue
                    (`WidgetLayoutLibrary.RemoveAllWidgets`)
                    (`self.DisableInput` _returnvalue_7 _returnvalue_6)
                    (`self.K2_SetActorRotation` _returnvalue_7 (struct :`Yaw` -180.0) false)
                    (`GameplayStatics.PlaySoundAtLocation` "/Game/Audio/Dialogue/4thInteraction/Donavon4thDialogue.Donavon4thDialogue" (`self.K2_GetActorLocation`) (struct) 1.0 1.0 0.0 null null null)
                    (`KismetSystemLibrary.Delay` 11.0)
                    (`self.EnableInput` _returnvalue_7 _returnvalue_6)
                    (set `self.4thDialogue` true)
                    (else
                      ;[0 1 0.2044] 3rdDialogue
                      (`WidgetLayoutLibrary.RemoveAllWidgets`)
                      (`self.DisableInput` _returnvalue_5 _returnvalue_4)
                      (`self.K2_SetActorRotation` _returnvalue_5 (struct :`Yaw` -180.0) false)
                      (`GameplayStatics.PlaySoundAtLocation` "/Game/Audio/Dialogue/3rdInteraction/Donavon3rdDialogue.Donavon3rdDialogue" (`self.K2_GetActorLocation`) (struct) 1.0 1.0 0.0 null null null)
                      (`KismetSystemLibrary.Delay` 12.0)
                      (`self.EnableInput` _returnvalue_5 _returnvalue_4)
                      (set `self.3rdDialogue` true)))
                  (else
                    ;[0 1 0.07217] 2ndDialogue
                    (`WidgetLayoutLibrary.RemoveAllWidgets`)
                    (`self.DisableInput` _returnvalue_3 _returnvalue_2)
                    (`self.K2_SetActorRotation` _returnvalue_3 (struct :`Yaw` -180.0) false)
                    (`GameplayStatics.PlaySoundAtLocation` "/Game/Audio/Dialogue/2ndInteraction/Donavon2ndDialogue.Donavon2ndDialogue" (`self.K2_GetActorLocation`) (struct) 1.0 1.0 0.0 null null null)
                    (`KismetSystemLibrary.Delay` 22.0)
                    (`self.EnableInput` _returnvalue_3 _returnvalue_2)
                    (set `self.2ndDialogue` true))))
              (else
                ;[0 1 0.0311] 1stDialogue
                (`WidgetLayoutLibrary.RemoveAllWidgets`)
                (`self.DisableInput` _returnvalue _returnvalue_8)
                (`self.K2_SetActorRotation` _returnvalue (struct :`Yaw` -180.0) false)
                (`GameplayStatics.PlaySoundAtLocation` "/Game/Audio/Dialogue/1stInteraction/Donavon1stDialogue.Donavon1stDialogue" (`self.K2_GetActorLocation`) (struct) 1.0 1.0 0.0 null null null)
                (`KismetSystemLibrary.Delay` 16.0)
                (`self.EnableInput` _returnvalue _returnvalue_8)))))))))

(event `Reset Interact`
  ;[1 1 1] Interact
  (`|ExecutionSequence`
    (:`then_0`
      (if (`self.KnifeFound`)
        (goto _label :!via `Reset`)))
    (:`then_1`
      (if (`self.GlovesFound`)
        (goto _label :!via `Reset`)))
    (:`then_2`
      (if (`self.RagFound`)
        (goto _label :!via `Reset`)))))

(event `self.Box.OnComponentBeginOverlap`
  (params (OverlappedComponent :type "PrimitiveComponent Object Reference") (OtherActor :type "Actor Object Reference") (OtherComp :type "PrimitiveComponent Object Reference") (OtherBodyIndex :type Integer) (bFromSweep :type Boolean) (SweepResult :type "HitResult Structure (by ref)"))
  (bind _returnvalue (`GameplayStatics.GetPlayerController` 0))
  ;[1 1 1] TriggerBox
  (cast `/Game/Character/BP_StoryAdv_Character` OtherActor)
  (`self.EnableInput` _returnvalue)
  (if (`self.1stDialogue`)
    (if (`self.KnifeFound`)
      (bind _returnvalue_2 (`|CreateWidget` "/Game/Widgets/Interactable_Widget.Interactable_Widget_C" _returnvalue :!label _label_3))
      (bind _output_get (set `self.InteractableWidget` _returnvalue_2))
      (`UserWidget.AddToViewport` _output_get 0)
      (`self.Reset Interact`)
      (goto _label_2 :!via `Open`))
    (else
      (goto _label_3))))

(event `self.Box.OnComponentEndOverlap`
  (params (OverlappedComponent :type "PrimitiveComponent Object Reference") (OtherActor :type "Actor Object Reference") (OtherComp :type "PrimitiveComponent Object Reference") (OtherBodyIndex :type Integer))
  ;[1 1 1] TriggerBox
  (cast `/Game/Character/BP_StoryAdv_Character` OtherActor)
  (`Widget.RemoveFromParent` (`self.InteractableWidget`))
  (goto _label_2 :!via `Close`))

(event `self.ReceiveTick`
  (params (DeltaSeconds :type "Float (single-precision)"))
  ;[1 1 1] CheckPlayerBools
  (bind _asbp_story_adv_character (cast `/Game/Character/BP_StoryAdv_Character` (`GameplayStatics.GetPlayerCharacter` 0)))
  (if (`/Game/Character/BP_StoryAdv_Character.FoundKnife` _asbp_story_adv_character)
    (set `self.1stDialogue` true)
    (set `self.KnifeFound` true)
    (if (`/Game/Character/BP_StoryAdv_Character.FoundGloves` _asbp_story_adv_character)
      (set `self.2ndDialogue` true)
      (set `self.GlovesFound` true)
      (if (`/Game/Character/BP_StoryAdv_Character.FoundRag` _asbp_story_adv_character)
        (set `self.RagFound` true)
        (set `self.3rdDialogue` true)))))

(fn `UserConstructionScript`)