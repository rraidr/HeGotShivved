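; Lara NPC Blueprint that plays her fourth dialogue and advances the story once the player has found the rag.
; Tick polls the story character's FoundRag flag; when set, entering the box shows an interact widget and opens a gate that leaving closes.
; A one-time interact press clears widgets, disables player input, rotates the player and plays the line, then sets FoundKIller on the character after a fixed delay.
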(event `InputAction|Interact` :consume false
  (params (Key :type "Key Structure"))
  (bind _returnvalue (`GameplayStatics.GetPlayerCharacter` 0))
  (:`Pressed`
    (if (`self.FoundRag`)
      (`/Engine/EditorBlueprintResources/StandardMacros.DoOnce` false
        (:`Completed`
          (`/Engine/EditorBlueprintResources/StandardMacros.Gate` true :!label _label
            (:`Exit`
              (`WidgetLayoutLibrary.RemoveAllWidgets`)
              (`self.DisableInput` _returnvalue (`GameplayStatics.GetPlayerController` 0))
              (`self.K2_SetActorRotation` _returnvalue (struct :`Yaw` 160.0) false)
              (`GameplayStatics.PlaySoundAtLocation` "/Game/Audio/Dialogue/4thInteraction/Lara4thDialogue.Lara4thDialogue" (`self.K2_GetActorLocation`) (struct) 1.0 1.0 0.0 null null null)
              (`KismetSystemLibrary.Delay` 18.0)
              (bind _asbp_story_adv_character (cast `/Game/Character/BP_StoryAdv_Character` (`GameplayStatics.GetPlayerCharacter` 0)))
              (set `/Game/Character/BP_StoryAdv_Character.FoundKIller` true _asbp_story_adv_character))))))))

(event `self.Box.OnComponentBeginOverlap`
  (params (OverlappedComponent :type "PrimitiveComponent Object Reference") (OtherActor :type "Actor Object Reference") (OtherComp :type "PrimitiveComponent Object Reference") (OtherBodyIndex :type Integer) (bFromSweep :type Boolean) (SweepResult :type "HitResult Structure (by ref)"))
  (bind _returnvalue (`GameplayStatics.GetPlayerController` 0))
  (cast `/Game/Character/BP_StoryAdv_Character` OtherActor)
  (`self.EnableInput` _returnvalue)
  (if (`self.FoundRag`)
    (bind _returnvalue_2 (`|CreateWidget` "/Game/Widgets/Interactable_Widget.Interactable_Widget_C" _returnvalue))
    (bind _output_get (set `self.InteractableWidget` _returnvalue_2))
    (`UserWidget.AddToViewport` _output_get 0)
    (goto _label :!via `Open`)))

(event `self.Box.OnComponentEndOverlap`
  (params (OverlappedComponent :type "PrimitiveComponent Object Reference") (OtherActor :type "Actor Object Reference") (OtherComp :type "PrimitiveComponent Object Reference") (OtherBodyIndex :type Integer))
  (cast `/Game/Character/BP_StoryAdv_Character` OtherActor)
  (`Widget.RemoveFromParent` (`self.InteractableWidget`))
  (goto _label :!via `Close`))

(event `self.ReceiveTick`
  (params (DeltaSeconds :type "Float (single-precision)"))
  (bind _asbp_story_adv_character (cast `/Game/Character/BP_StoryAdv_Character` (`GameplayStatics.GetPlayerCharacter` 0)))
  (if (`/Game/Character/BP_StoryAdv_Character.FoundRag` _asbp_story_adv_character)
    (set `self.FoundRag` true)))

(fn `UserConstructionScript`)